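; Cricket spin-bowler ball actor that delivers itself on spawn and expires after ten seconds.
; BeginPlay randomly picks off or leg spin, setting line and signed spin magnitude, then launches the mesh with a randomized impulse.
; The first pitch hit during delivery applies sideways turn via an impulse along velocity crossed with up, then ends delivery.
; Ground hits after delivery set HasBounced.
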(event EventBeginPlay
  (Actor|SetLifeSpan 1e+01)
  ;[1 1 1] Delivery Line and Length
  ;;[1 1 1] Derive Line From Spin Type (1- OffSpin/ 0-LegSpin)
  (bind _output_get (Variables|Default|SetspinType (Math|Random|RandomBool)))
  (if _output_get
    ;;;[1 1 1] Off Spin
    (Variables|Default|SetSpinMag (Math|Float|Truncate (Math|Random|RandomFloatinRange -1.5e+02 -1e+02)))
    (Variables|Default|SetLine%28Y%29 0)
    (else
      ;;;[1 1 1] Leg Spin
      (Variables|Default|SetSpinMag (Math|Float|Truncate (Math|Random|RandomFloatinRange 1e+02 1.5e+02)))
      (Variables|Default|SetLine%28Y%29 -50)))
  (Physics|AddImpulse (Variables|Debug|GetStaticMeshComponent) (Math|Vector|MakeVector (Math|Random|RandomFloatinRange -9.5e+02 -1.2e+03) (Math|Conversions|ToFloat(Integer) (Variables|Default|GetLine%28Y%29)) (Math|Random|RandomFloatinRange 7e+01 1.2e+02)) "None" false))

(event Collision|EventActorBeginOverlap
  (params (OtherActor :type Actor%20Object%20Reference)))

(event Collision|EventHit
  (params (MyComp :type Primitive%20Component%20Object%20Reference) (Other :type Actor%20Object%20Reference) (OtherComp :type Primitive%20Component%20Object%20Reference) (bSelfMoved :type Boolean) (HitLocation :type Vector :default "0, 0, 0") (HitNormal :type Vector :default "0, 0, 0") (NormalImpulse :type Vector :default "0, 0, 0") (Hit :type Hit%20Result%20Structure%20%28by%20ref%29))
  ;[1 1 1] On Hit
  (Utilities|FlowControl|Sequence
    (:then_0
      (if (Components|ComponentHasTag OtherComp "Ground")
        (if (not (Variables|Default|GetinDelivery))
          (Variables|Default|SethasBounced true))))
    (:then_1
      (if (Components|ComponentHasTag OtherComp "Pitch")
        (if (Variables|Default|GetinDelivery)
          (Physics|AddImpulse (Variables|Debug|GetStaticMeshComponent) (* (Math|Vector|Normalize (Math|Vector|CrossProduct (Transformation|GetVelocity) (Math|Vector|GetUpVector "0, 0, 0"))) (Math|Conversions|ToFloat(Integer) (Variables|Default|GetSpinMag))) "None" false)
          (Variables|Default|SetinDelivery false))))))

(fn ConstructionScript)