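; Cricket fielder character that chases a target, gathers the ball and detects catch dismissals.
; Each tick it updates its squared distance to the current target, then moves toward it on the ground plane when active or stops when inactive.
; Overlapping a ball sets possession, and the ball's second tag selects the spin, seam or swing cast; an unbounced ball flags Out.
; ResetField teleports the fielder back to its starting position.
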(event EventBeginPlay
  (Variables|Default|SetinitialPos (Transformation|GetActorLocation)))

(event Collision|EventActorBeginOverlap
  (params (OtherActor :type Actor%20Object%20Reference))
  (if (Actor|ActorHasTag OtherActor "Ball")
    (Variables|Default|SethasBall true)
    (switch string (Utilities|String|ToString(Name) (Utilities|Array|Get(acopy) (Variables|/Script/Engine.Actor|GetTags OtherActor) 1))
      (:Spin
        (bind _asspin_ball_blueprint (Utilities|Casting|CastToSpinBall_Blueprint OtherActor))
        (if (not (Variables|/Game/TrialCricket/Blueprints/SpinBall_Blueprint.SpinBall_Blueprint_C|GethasBounced _asspin_ball_blueprint))
          (Variables|Default|Setout true :!label _label)))
      (:Seam
        (bind _asseam_ball_blueprint (Utilities|Casting|CastToSeamBall_Blueprint OtherActor))
        (if (not (Variables|/Game/TrialCricket/Blueprints/SeamBall_Blueprint.SeamBall_Blueprint_C|GethasBounced _asseam_ball_blueprint))
          (goto _label)))
      (:Swing
        (bind _asswing_ball_blueprint (Utilities|Casting|CastToSwingBall_Blueprint OtherActor))
        (if (not (Variables|/Game/TrialCricket/Blueprints/SwingBall_Blueprint.SwingBall_Blueprint_C|GethasBounced _asswing_ball_blueprint))
          (goto _label))))))

(event EventTick
  (params (DeltaSeconds :type Float%20%28single-precision%29))
  (bind _currenttarget (Variables|Default|GetcurrentTarget))
  (bind _returnvalue (Transformation|GetActorLocation _currenttarget))
  (bind (_x _y) (Math|Vector|BreakVector _returnvalue))
  (Utilities|IsValid _currenttarget
    (:Is%20Valid
      (Variables|Default|SetDistance (Math|Float|Truncate (Transformation|GetSquaredDistanceTo _currenttarget)))
      (if (Variables|Default|Getactive)
        (AI|Navigation|SimpleMovetoLocation (Pawn|GetController) (Math|Vector|MakeVector _x _y 0.0))
        (else
          (Components|Movement|StopMovementImmediately (Variables|Character|GetCharacterMovement)))))))

(fn ConstructionScript)

(fn ResetField
  (Transformation|SetActorLocation (Variables|Default|GetinitialPos) false true))