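; Cricket ball actor that bowls itself as a randomized swing delivery on spawn and expires after a fixed lifespan.
; BeginPlay picks in- or out-swing and an occasional bouncer, which set the line, swing strength and launch impulse.
; Tick applies sideways physics force while InDelivery, creating swing until the ball hits a Pitch-tagged component.
; Hits on Ground-tagged components after the delivery ends set HasBounced.
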(event EventBeginPlay
  (Actor|SetLifeSpan 1e+01)
  ;[1 1 1] Delivery Line and Length
  ;;[1 1 1] Derive Line From Swing Type (1- In Swing/ 0-Out Swing)
  (bind _output_get (Variables|Default|SetSwingType (Math|Random|RandomBool)))
  (if _output_get
    ;;;[1 1 1] In Swing
    (Variables|Default|SetSwingMag (Math|Float|Truncate (Math|Random|RandomFloatinRange -4e+02 -3e+02)))
    ;;;[1 1 1] Is Bouncer?
    (bind _output_get_2 (Variables|Default|SetisBouncer (Math|Random|RandomBoolwithWeight 0.1)))
    (if _output_get_2
      (Variables|Default|SetLine%28Y%29 20)
      ;;[1 1 1] Line & Speed
      ;;;[1 1 1] Bouncer
      (Variables|Default|Setimpulse (Math|Vector|MakeVector (Math|Random|RandomFloatinRange -1.9e+03 -1.7e+03) (Math|Conversions|ToFloat(Integer) (Variables|Default|GetLine%28Y%29)) (Math|Random|RandomFloatinRange -5e+02 -3e+02)) :!label _label)
      (else
        (Variables|Default|SetLine%28Y%29 115)
        ;;;[1 1 1] Length Delivery
        (Variables|Default|Setimpulse (Math|Vector|MakeVector (Math|Random|RandomFloatinRange -1.3e+03 -1.4e+03) (Math|Conversions|ToFloat(Integer) (Variables|Default|GetLine%28Y%29)) (Math|Random|RandomFloatinRange -5e+01 0.0)) :!label _label_2)))
    (else
      ;;;[1 1 1] Out Swing
      (Variables|Default|SetSwingMag (Math|Float|Truncate (Math|Random|RandomFloatinRange 3e+02 4e+02)))
      ;;;[1 1 1] Is Bouncer?
      (bind _output_get_3 (Variables|Default|SetisBouncer (Math|Random|RandomBoolwithWeight 0.1)))
      (if _output_get_3
        (Variables|Default|SetLine%28Y%29 -110)
        (goto _label)
        (else
          (Variables|Default|SetLine%28Y%29 -165)
          (goto _label_2)))))
  (Physics|AddImpulse (Variables|Debug|GetStaticMeshComponent) (Variables|Default|Getimpulse) "None" false))

(event Collision|EventActorBeginOverlap
  (params (OtherActor :type Actor%20Object%20Reference)))

(event Collision|EventHit
  (params (MyComp :type Primitive%20Component%20Object%20Reference) (Other :type Actor%20Object%20Reference) (OtherComp :type Primitive%20Component%20Object%20Reference) (bSelfMoved :type Boolean) (HitLocation :type Vector :default "0, 0, 0") (HitNormal :type Vector :default "0, 0, 0") (NormalImpulse :type Vector :default "0, 0, 0") (Hit :type Hit%20Result%20Structure%20%28by%20ref%29))
  ;[1 1 1] On Hit
  (Utilities|FlowControl|Sequence
    (:then_0
      (if (Components|ComponentHasTag OtherComp "Ground")
        (if (not (Variables|Default|GetinDelivery))
          (Variables|Default|SethasBounced true))))
    (:then_1
      (if (Components|ComponentHasTag OtherComp "Pitch")
        (if (Variables|Default|GetinDelivery)
          (Variables|Default|SetinDelivery false))))))

(event EventTick
  (params (DeltaSeconds :type Float%20%28single-precision%29))
  ;[1 1 1] Swing Bowling
  (if (Variables|Default|GetinDelivery)
    (Physics|AddForce (Variables|Debug|GetStaticMeshComponent) (Math|Vector|MakeVector 0.0 (Math|Conversions|ToFloat(Integer) (Variables|Default|GetSwingMag)) 0.0) "None" false)))

(fn ConstructionScript)