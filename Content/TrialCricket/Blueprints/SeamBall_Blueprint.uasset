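; SeamBall is a cricket delivery actor that launches itself on spawn as a seam-bowled ball and expires after a short lifespan.
; BeginPlay randomly picks off or leg seam, setting line and seam strength, then applies a physics impulse for either a length ball or an occasional bouncer.
; The first pitch hit during delivery adds sideways seam movement perpendicular to velocity and ends the delivery phase; later ground hits set HasBounced.
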(event Collision|EventActorBeginOverlap
  (params (OtherActor :type Actor%20Object%20Reference)))

(event Collision|EventHit
  (params (MyComp :type Primitive%20Component%20Object%20Reference) (Other :type Actor%20Object%20Reference) (OtherComp :type Primitive%20Component%20Object%20Reference) (bSelfMoved :type Boolean) (HitLocation :type Vector :default "0, 0, 0") (HitNormal :type Vector :default "0, 0, 0") (NormalImpulse :type Vector :default "0, 0, 0") (Hit :type Hit%20Result%20Structure%20%28by%20ref%29))
  ;[1 1 1] On Hit
  (Utilities|FlowControl|Sequence
    (:then_0
      (if (Components|ComponentHasTag OtherComp "Ground")
        (if (not (Variables|Default|GetinDelivery))
          (Variables|Default|SethasBounced true))))
    (:then_1
      (if (Components|ComponentHasTag OtherComp "Pitch")
        (if (Variables|Default|GetinDelivery)
          (Physics|AddImpulse (Variables|Debug|GetStaticMeshComponent) (* (Math|Vector|Normalize (Math|Vector|CrossProduct (Transformation|GetVelocity) (Math|Vector|GetUpVector "0, 0, 0"))) (Math|Conversions|ToFloat(Integer) (Variables|Default|GetSeamMag))) "None" false)
          (Variables|Default|SetinDelivery false))))))

(event EventBeginPlay
  (Actor|SetLifeSpan 1e+01)
  ;[1 1 1] Delivery Line and Length
  ;;[1 1 1] Derive Line From Seam Type (1- OffSeam/ 0-LegSeam)
  (bind _output_get (Variables|Default|SetSeamType (Math|Random|RandomBool)))
  (if _output_get
    ;;;[1 1 1] Off Seam
    (Variables|Default|SetSeamMag (Math|Float|Truncate (Math|Random|RandomFloatinRange -4e+01 -6e+01)))
    (Variables|Default|SetLine%28Y%29 -10)
    (else
      ;;;[1 1 1] Leg Seam
      (Variables|Default|SetSeamMag (Math|Float|Truncate (Math|Random|RandomFloatinRange 4e+01 6e+01)))
      (Variables|Default|SetLine%28Y%29 -60)))
  ;;;[1 1 1] Is Bouncer?
  (bind _output_get_2 (Variables|Default|SetisBouncer (Math|Random|RandomBoolwithWeight 0.1)))
  (if _output_get_2
    ;;[1 1 1] Line & Speed
    ;;;[1 1 1] Bouncer
    (Variables|Default|Setimpulse (Math|Vector|MakeVector (Math|Random|RandomFloatinRange -1.9e+03 -1.7e+03) (Math|Conversions|ToFloat(Integer) (Variables|Default|GetLine%28Y%29)) (Math|Random|RandomFloatinRange -5e+02 -3e+02)))
    (else
      ;;;[1 1 1] Length Delivery
      (Variables|Default|Setimpulse (Math|Vector|MakeVector (Math|Random|RandomFloatinRange -1.4e+03 -1.6e+03) (Math|Conversions|ToFloat(Integer) (Variables|Default|GetLine%28Y%29)) (Math|Random|RandomFloatinRange -1e+02 0.0)))))
  (Physics|AddImpulse (Variables|Debug|GetStaticMeshComponent) (Variables|Default|Getimpulse) "None" false))

(fn ConstructionScript)